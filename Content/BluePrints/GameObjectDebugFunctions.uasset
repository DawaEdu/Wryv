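; GameObjectDebugFunctions is a set of debug drawing helpers that visualize a GameObject in the world.
; DrawSightRange draws a single-frame cylinder with the sight range from Stats as its radius, rising from the object's position by its HitBox's scaled Z extent.
; DrawDebugText prints the object's ToString output as a debug string at its position.
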(fn `DrawDebugText`
  (params (GameObject :type "GameObject Object Reference"))
  (bind _returnvalue (`GameObject.ToString` GameObject))
  (`KismetSystemLibrary.DrawDebugString` null (`GameObject.Pos` GameObject) _returnvalue))

(fn `DrawSightRange`
  (params (GameObject :type "GameObject Object Reference"))
  (bind _pos (`GameObject.Pos` GameObject))
  (`KismetSystemLibrary.DrawDebugCylinder` null _pos (+ (* (`BoxComponent.GetScaledBoxExtent` (`GameObject.hitBox` GameObject)) (0.0 0.0 1.0)) _pos) (`.SightRange` (break `UnitsData` (`GameObject.Stats` GameObject))) 24 (struct :`R` 1.0 :`G` 1.0 :`B` 1.0 :`A` 1.0) 0.0))